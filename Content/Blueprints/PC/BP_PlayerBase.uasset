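; Base player Blueprint that maps Enhanced Input dash and guard actions to inherited or external functions.
; Dash Triggered raises movement speed and Completed lowers it, while Canceled plays a montage-driven dash with force.
; Guard Triggered and Completed start and end guarding, while Canceled performs a perfect guard, splitting each action by trigger state.
; Move and Look events are empty, with their older movement and camera nodes left disconnected.
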(event Input|EnhancedActionEvents|EnhancedInputActionIA_Move
  (params (ActionValue :type Vector%202D%20Structure) (ElapsedSeconds :type Float%20%28double-precision%29) (TriggeredSeconds :type Float%20%28double-precision%29) (InputAction :type Input%20Action%20Object%20Reference :default "/Game/Input/Actions/IA_Move.IA_Move"))
  ;[0.15 0.15 0.15 0.5] Comment
)

(event Input|EnhancedActionEvents|EnhancedInputActionIA_Look
  (params (ActionValue :type Vector%202D%20Structure) (ElapsedSeconds :type Float%20%28double-precision%29) (TriggeredSeconds :type Float%20%28double-precision%29) (InputAction :type Input%20Action%20Object%20Reference :default "/Game/Input/Actions/IA_Look.IA_Look"))
  ;[0.15 0.15 0.15 0.5] Comment
)

(event Input|EnhancedActionEvents|EnhancedInputActionIA_Dash
  (params (ActionValue :type Boolean) (ElapsedSeconds :type Float%20%28double-precision%29) (TriggeredSeconds :type Float%20%28double-precision%29) (InputAction :type Input%20Action%20Object%20Reference :default "/Game/Input/Actions/IA_Dash.IA_Dash"))
  (:Triggered
    (Class|PlayerCharacterBase|SetMovemoentSpeed 6e+02))
  (:Canceled
    (Class|PlayerCharacterBase|Dash "/Game/Animations/PlayerBaseABP/Dash/AM_PCBaseDash.AM_PCBaseDash" 5e+03))
  (:Completed
    (Class|PlayerCharacterBase|SetMovemoentSpeed 3e+02)))

(event Input|EnhancedActionEvents|EnhancedInputActionIA_Guard
  (params (ActionValue :type Boolean) (ElapsedSeconds :type Float%20%28double-precision%29) (TriggeredSeconds :type Float%20%28double-precision%29) (InputAction :type Input%20Action%20Object%20Reference :default "/Game/Input/Actions/IA_Guard.IA_Guard"))
  (:Triggered
    (Class|PlayerCharacterBase|StartGuard 1.5e+02))
  (:Canceled
    (Class|PlayerCharacterBase|PerfectGuard "/Game/Animations/PlayerBaseABP/Guard/AM_PCBaseGuard.AM_PCBaseGuard"))
  (:Completed
    (Class|PlayerCharacterBase|EndGuard 3e+02)))

(event EventBeginPlay)

(event Collision|EventActorBeginOverlap
  (params (OtherActor :type Actor%20Object%20Reference)))

(event EventTick
  (params (DeltaSeconds :type Float%20%28single-precision%29))
  ;[0.15 0.15 0.15 0.5] Comment
)

(event Input|KeyboardEvents|DebugKeyP
  (params (Key :type Key%20Structure :default "None") (ActionValue :type Input%20Action%20Value%20Structure)))

(fn ConstructionScript)